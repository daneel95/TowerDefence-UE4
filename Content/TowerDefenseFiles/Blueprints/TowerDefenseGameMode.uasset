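; Game mode for a tower defense game that holds the level state: money, lives, checkpoints, wave counter and enemy list.
; LevelConstantsSetter initializes that state, and helper functions handle turret prices, checkpoint lookup and money and life changes, with a HUD warning when funds are short.
; SpawnNextWave starts a looping timer that spawns enemies from the array at the first checkpoint.
; Tick stops that timer once the wave's last index is reached.
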(event `self.ReceiveBeginPlay`)

(event `self.ReceiveTick`
  (params (DeltaSeconds :type "Float (single-precision)"))
  ;[1 1 1] Check if wave should be stopped and stop it if true
  (if (`self.Spawning`)
    (if (== (`self.EnemyToSpawnIndex`) (`self.EnemyToSpawnIndexAfterWave`))
      (`self.StopWave`))))

(fn `AddMoney`
  (params (Reward :type Integer))
  (set `self.Money` (+ Reward (`self.Money`))))

(fn `GetCheckpoint`
  (params (CheckpointIndex :type Integer))
  (returns (Checkpoint :type "Vector Structure"))
  (return (+ (`|GetArrayItem` (`self.CheckPoints`) CheckpointIndex) (`KismetMathLibrary.MakeVector` 0.0 0.0 (`self.CheckpointZOverhead`)))))

(fn `GetTurretPrice`
  (params (TurretType :type "/Game/TowerDefenseFiles/Blueprints/Auxiliary/TurretTypes_Enum Enum" :default "NewEnumerator0"))
  (returns (TurretBuildPrice :type Integer))
  (return (select `/Game/TowerDefenseFiles/Blueprints/Auxiliary/TurretTypes_Enum` TurretType :`NewEnumerator1` 100 :`NewEnumerator2` 150 :`NewEnumerator3` 300)))

(fn `LevelConstantsSetter`
  (params (CheckPoints :type "Array of Vector Structure") (Lives :type Integer) (StartingMoney :type Integer) (EnemiesArray :type "Array of /Game/TowerDefenseFiles/Blueprints/Enemy/BaseEnemy_BP Class Reference") (NumberOfWaves :type Integer) (NumberOfEnemiesPerWave :type "Array of Integer"))
  (set `self.EnemyToSpawnIndex` 0)
  (set `self.EnemyToSpawnIndexAfterWave` 0)
  (set `self.CurrentWave` 0)
  (set `self.Spawning` false)
  (bind _output_get (set `self.CheckPoints` CheckPoints))
  (set `self.Lives` Lives)
  (set `self.Money` StartingMoney)
  (set `self.EnemiesArray` EnemiesArray)
  (set `self.NumberOfWaves` NumberOfWaves)
  (set `self.NumberOfEnemiesPerWave` NumberOfEnemiesPerWave)
  (set `self.NumberOfCheckpoints` (`KismetArrayLibrary.Array_Length` _output_get)))

(fn `SpawnNextEnemy`
  (`|SpawnActorFromClass` (`|GetArrayItem` (`self.EnemiesArray`) (`self.EnemyToSpawnIndex`)) (`KismetMathLibrary.MakeTransform` (+ (`|GetArrayItem` (`self.CheckPoints`)) (`KismetMathLibrary.MakeVector` 0.0 0.0 (`self.CheckpointZOverhead`))) (struct) (0.7 0.7 0.7)) "Undefined" "OverrideRootScale" null null)
  (set `self.EnemyToSpawnIndex` (+ (`self.EnemyToSpawnIndex`) 1))
  (set `self.Spawning` true))

(fn `SpawnNextWave`
  (params (NumberOfEnemiesToSpawn :type Integer))
  (set `self.CurrentWave` (+ (`self.CurrentWave`) 1))
  (set `self.EnemyToSpawnIndexAfterWave` (+ NumberOfEnemiesToSpawn (`self.EnemyToSpawnIndex`)))
  (`KismetSystemLibrary.K2_SetTimer` null "SpawnNextEnemy" 1.0 true))

(fn `StopWave`
  (set `self.Spawning` false)
  (`KismetSystemLibrary.K2_ClearTimer` null "SpawnNextEnemy"))

(fn `SubstractLives`
  (params (LivesToSubstract :type Integer :default 1))
  (set `self.Lives` (- (`self.Lives`) LivesToSubstract)))

(fn `SubstractMoney`
  (params (MoneyToSubstract :type Integer))
  (returns (Success :type Boolean))
  (bind _returnvalue (- (`self.Money`) MoneyToSubstract))
  (if (>= _returnvalue 0)
    (set `self.Money` _returnvalue)
    (return true)
    (else
      (bind _astower_defense_controller (cast `/Game/TowerDefenseFiles/Blueprints/TowerDefenseController` (`GameplayStatics.GetPlayerController` 0)))
      (bind _astower_defense_hud (cast `/Game/TowerDefenseFiles/Blueprints/TowerDefenseHud` (`PlayerController.GetHUD` _astower_defense_controller)))
      (`/Game/TowerDefenseFiles/Blueprints/TowerDefenseHud.ShowMainUIMessage` _astower_defense_hud "Not enough money!")
      (return false))))

(fn `UserConstructionScript`)