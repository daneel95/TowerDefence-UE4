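; Tower defense tile actor that acts as an empty build spot or, once its turret type is set, a working turret.
; Clicking opens the build widget or the info widget with a range decal.
; BuildTurret charges the game mode's money and replaces the tile with the chosen turret Blueprint.
; On Tick, turrets take the first enemy in range, rotate toward it and fire projectiles from random tips, throttled by fire rate.
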(event `self.ReceiveBeginPlay`)

(event `self.ReceiveTick`
  (params (DeltaSeconds :type "Float (single-precision)"))
  ;[1 1 1] Check if there is an enemy withing range. If not continue searching
  (if (`|EnumInequality` (`self.TurretType`) "NewEnumerator0")
    (if (`KismetSystemLibrary.IsValid` (`self.EnemyWithinRange`))
      ;[1 1 1] Check if enemy still in range
      (`self.CheckEnemyStillInRange`)
      (if (`KismetSystemLibrary.IsValid` (`self.EnemyWithinRange`))
        (`|ExecutionSequence`
          (:`then_0`
            ;[1 1 1] Fire at a given fire rate
            (if (`self.CanFire`)
              (`self.Fire` (`self.TurretTips`))
              (set `self.CanFire` false)
              (`KismetSystemLibrary.Delay` (/ 1.0 (`self.FireRate`)))
              (set `self.CanFire` true)))
          (:`then_1`
            ;[1 1 1] Rotate turret top
            (`SceneComponent.K2_SetWorldRotation` (`self.TurretTop`) (`KismetMathLibrary.FindLookAtRotation` (`SceneComponent.K2_GetComponentLocation` (`self.TurretTop`)) (`SceneComponent.K2_GetComponentLocation` (`Actor.RootComponent` (`self.EnemyWithinRange`)))) false false))))
      (else
        (`self.GetEnemyWithinRange`)))))

(event `self.Tile.OnClicked`
  (params (TouchedComponent :type "PrimitiveComponent Object Reference") (ButtonPressed :type "Key Structure"))
  ;[1 1 1] When clicking on tile open build UI and play animation
  (if (`|EnumEquality` (`self.TurretType`) "NewEnumerator0")
    (bind _astower_defense_controller (cast `/Game/TowerDefenseFiles/Blueprints/TowerDefenseController` (`GameplayStatics.GetPlayerController` 0)))
    (bind _astower_defense_hud (cast `/Game/TowerDefenseFiles/Blueprints/TowerDefenseHud` (`PlayerController.GetHUD` _astower_defense_controller)))
    (bind _turretinformationwidget (`/Game/TowerDefenseFiles/Blueprints/TowerDefenseHud.TurretInformationWidget` _astower_defense_hud))
    (`/Game/TowerDefenseFiles/Blueprints/Widgets/TurretInformation_WB.HideUI` _turretinformationwidget)
    (`Widget.SetVisibility` _turretinformationwidget "Hidden")
    (bind _turretbuildwidget (`/Game/TowerDefenseFiles/Blueprints/TowerDefenseHud.TurretBuildWidget` _astower_defense_hud))
    (`Widget.SetVisibility` _turretbuildwidget "SelfHitTestInvisible")
    (set `/Game/TowerDefenseFiles/Blueprints/Widgets/TurretBuild_Widget.TurretTile` self _turretbuildwidget)
    (`UserWidget.PlayAnimation` _turretbuildwidget (`/Game/TowerDefenseFiles/Blueprints/Widgets/TurretBuild_Widget.TransitionAnimation` _turretbuildwidget) 0.0 1 "Forward" 1.0)
    (else
      ;[1 1 1] Hide widgets that are already up
      (bind _astower_defense_controller_2 (cast `/Game/TowerDefenseFiles/Blueprints/TowerDefenseController` (`GameplayStatics.GetPlayerController` 0) :!label _label))
      (bind _astower_defense_hud_2 (cast `/Game/TowerDefenseFiles/Blueprints/TowerDefenseHud` (`PlayerController.GetHUD` _astower_defense_controller_2)))
      (`Widget.SetVisibility` (`/Game/TowerDefenseFiles/Blueprints/TowerDefenseHud.TurretBuildWidget` _astower_defense_hud_2) "Hidden")
      (bind _turretinformationwidget_2 (`/Game/TowerDefenseFiles/Blueprints/TowerDefenseHud.TurretInformationWidget` _astower_defense_hud_2))
      ;[1 1 1] Hide Information Widget (Mainly because of range indicator)
      (`/Game/TowerDefenseFiles/Blueprints/Widgets/TurretInformation_WB.HideUI` _turretinformationwidget_2)
      ;[1 1 1] Spawn range indicator if it's not spawned already
      (if (not (`KismetSystemLibrary.IsValid` (`self.DecalRangeIndicator`)))
        (`self.SpawnRangeIndicator`))
      ;[1 1 1] Set Information Widget visibility + Render information + Play its animation
      (`Widget.SetVisibility` _turretinformationwidget_2 "SelfHitTestInvisible")
      (`/Game/TowerDefenseFiles/Blueprints/Widgets/TurretInformation_WB.RenderAllInformation` _turretinformationwidget_2 (`self.TurretType`) self)
      (`UserWidget.PlayAnimation` _turretinformationwidget_2 (`/Game/TowerDefenseFiles/Blueprints/Widgets/TurretInformation_WB.TransitionAnimation` _turretinformationwidget_2) 0.0 1 "Forward" 1.0))))

(event `self.TurretTop.OnClicked`
  (params (TouchedComponent :type "PrimitiveComponent Object Reference") (ButtonPressed :type "Key Structure"))
  ;[1 1 1] Register clicks anywhere on the object
  (goto _label))

(event `self.TurretBot.OnClicked`
  (params (TouchedComponent :type "PrimitiveComponent Object Reference") (ButtonPressed :type "Key Structure"))
  ;[1 1 1] Register clicks anywhere on the object
  (goto _label))

(fn `BuildTurret`
  (params (TurretType :type "/Game/TowerDefenseFiles/Blueprints/Auxiliary/TurretTypes_Enum Enum" :default "NewEnumerator0"))
  ;[1 1 1] If player has enough money spawn the given turret and destroy the tile
  (if (`|EnumInequality` TurretType "NewEnumerator0")
    (bind _astower_defense_game_mode (cast `/Game/TowerDefenseFiles/Blueprints/TowerDefenseGameMode` (`GameplayStatics.GetGameMode`)))
    (bind _turretbuildprice (`/Game/TowerDefenseFiles/Blueprints/TowerDefenseGameMode.GetTurretPrice` _astower_defense_game_mode TurretType))
    (bind _success (`/Game/TowerDefenseFiles/Blueprints/TowerDefenseGameMode.SubstractMoney` _astower_defense_game_mode _turretbuildprice))
    (if _success
      (`|SpawnActorFromClass` (select `/Game/TowerDefenseFiles/Blueprints/Auxiliary/TurretTypes_Enum` TurretType :`NewEnumerator1` "/Game/TowerDefenseFiles/Blueprints/Turrets/Turret0_BP.Turret0_BP_C" :`NewEnumerator2` "/Game/TowerDefenseFiles/Blueprints/Turrets/Turret1_BP.Turret1_BP_C" :`NewEnumerator3` "/Game/TowerDefenseFiles/Blueprints/Turrets/Turret2_BP.Turret2_BP_C" :!type "Actor Class Reference") (`self.GetTransform` self) "Undefined" "OverrideRootScale" null null)
      (`self.K2_DestroyActor`))))

(fn `CheckEnemyStillInRange`
  (if (not (< (`self.GetDistanceTo` self (`self.EnemyWithinRange`)) (`self.Range`)))
    (set `self.EnemyWithinRange` null)))

(fn `DestroyRangeIndicator`
  (bind _decalrangeindicator (`self.DecalRangeIndicator`))
  (if (`KismetSystemLibrary.IsValid` _decalrangeindicator)
    (`ActorComponent.K2_DestroyComponent` _decalrangeindicator)))

(fn `Fire`
  (params (TurretTips :type "Array of SceneComponent Object Reference"))
  ;[1 1 1] Takes a random turret tip to fire from
  (bind _asstatic_mesh_component (cast `StaticMeshComponent` (`|GetArrayItem` TurretTips (`KismetMathLibrary.RandomIntegerInRange` 0 (- (`KismetArrayLibrary.Array_Length` TurretTips) 1)))))
  (bind _returnvalue (`SceneComponent.K2_GetComponentLocation` _asstatic_mesh_component))
  ;[1 1 1] Spawn projectile. Set its rotation and position and set up it's variables
  (bind _returnvalue_2 (`|SpawnActorFromClass` (`self.ProjectileClass`) (`KismetMathLibrary.MakeTransform` _returnvalue (`KismetMathLibrary.FindLookAtRotation` _returnvalue (.location (`SceneComponent.GetRelativeTransform` (`/Game/TowerDefenseFiles/Blueprints/Enemy/BaseEnemy_BP.DefaultSceneRoot` (`self.EnemyWithinRange`))))) (0.1 0.1 0.1)) "Undefined" "OverrideRootScale" null null))
  (`self.SetUpProjectile` _returnvalue_2))

(fn `GetEnemyWithinRange`
  ;[1 1 1] Check if there is any ENEMY within turret range
  (bind _outactors (`GameplayStatics.GetAllActorsOfClass` "/Game/TowerDefenseFiles/Blueprints/Enemy/BaseEnemy_BP.BaseEnemy_BP_C"))
  (for _array_element _outactors
    (if (< (`self.GetDistanceTo` self _array_element) (`self.Range`))
      (set `self.EnemyWithinRange` _array_element)
      (break))))

(fn `MakeSetup`
  (params (Range :type "Float (double-precision)") (Damage :type Integer) (FireRate :type "Float (double-precision)") (TurretType :type "/Game/TowerDefenseFiles/Blueprints/Auxiliary/TurretTypes_Enum Enum" :default "NewEnumerator0") (TurretPrice :type Integer) (TurretTips :type "Array of SceneComponent Object Reference") (ProjectileClass :type "/Game/TowerDefenseFiles/Blueprints/Projectile/Projectile_BP Class Reference"))
  (set `self.Range` Range)
  (set `self.Damage` Damage)
  (set `self.FireRate` FireRate)
  (set `self.TurretType` TurretType)
  (set `self.TurretPrice` TurretPrice)
  (set `self.TurretTips` TurretTips)
  (set `self.ProjectileClass` ProjectileClass))

(fn `SetUpProjectile`
  (params (ProjectileToSetup :type "/Game/TowerDefenseFiles/Blueprints/Projectile/Projectile_BP Object Reference"))
  (set `/Game/TowerDefenseFiles/Blueprints/Projectile/Projectile_BP.Damage` (`self.Damage`) ProjectileToSetup)
  (set `/Game/TowerDefenseFiles/Blueprints/Projectile/Projectile_BP.Target` (`self.EnemyWithinRange`) ProjectileToSetup))

(fn `SpawnRangeIndicator`
  (bind _range (`self.Range`))
  (bind _returnvalue (`GameplayStatics.SpawnDecalAtLocation` (`self.RangeIndicator`) (`KismetMathLibrary.MakeVector` 10.0 _range _range) (`SceneComponent.K2_GetComponentLocation` (`self.Tile`))))
  (set `self.DecalRangeIndicator` _returnvalue))

(fn `UserConstructionScript`)