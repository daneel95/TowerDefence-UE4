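; Basic turret variant for the tower defense game, built on a parent turret class.
; On BeginPlay it reads range, damage, fire rate and price from the game mode's Turret0 stat map.
; It passes those stats to MakeSetup along with a turret type, BasicProjectile_BP and TurretTop's child components as firing tips.
; The Blueprint holds only this configuration, with no targeting or firing logic of its own.
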(event `self.ReceiveBeginPlay`
  (bind _astower_defense_game_mode (cast `/Game/TowerDefenseFiles/Blueprints/TowerDefenseGameMode` (`GameplayStatics.GetGameMode`)))
  (bind _turret0 (`/Game/TowerDefenseFiles/Blueprints/TowerDefenseGameMode.Turret0` _astower_defense_game_mode))
  (`self.MakeSetup` (`BlueprintMapLibrary.Map_Find` _turret0 "range") (`KismetMathLibrary.FTrunc` (`BlueprintMapLibrary.Map_Find` _turret0 "damage")) (`BlueprintMapLibrary.Map_Find` _turret0 "fire_rate") "NewEnumerator1" (`KismetMathLibrary.FTrunc` (`BlueprintMapLibrary.Map_Find` _turret0 "price")) (`SceneComponent.GetChildrenComponents` (`self.TurretTop`) false) "/Game/TowerDefenseFiles/Blueprints/Projectile/BasicProjectile_BP.BasicProjectile_BP_C"))

(fn `UserConstructionScript`
  (`parent.UserConstructionScript`))