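; Tower defense Game Instance Blueprint that provides helper functions for saving and loading game data in named slots.
; LoadData checks that the slot exists and returns its contents cast to SaveGame_BP, or returns without data if either step fails.
; SaveData writes the supplied object to the slot when it is empty, replacing an existing save only if Overwrite is set.
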(fn `LoadData`
  (params (FileName :type String :default "PlayerLevel"))
  (returns (RetrievedData :type "/Game/TowerDefenseFiles/Blueprints/SaveGame_BP Object Reference"))
  (bind _returnvalue (`GameplayStatics.DoesSaveGameExist` FileName))
  (if _returnvalue
    (bind _returnvalue_2 (`GameplayStatics.LoadGameFromSlot` FileName))
    (bind _assave_game_bp (cast `/Game/TowerDefenseFiles/Blueprints/SaveGame_BP` _returnvalue_2)
      (:`then`
        (return _assave_game_bp))
      (:`CastFailed`
        _)))
  (return null))

(fn `SaveData`
  (params (Data :type "/Game/TowerDefenseFiles/Blueprints/SaveGame_BP Object Reference") (FileName :type String :default "PlayerLevel") (Overwrite :type Boolean :default true))
  (bind _returnvalue (`GameplayStatics.DoesSaveGameExist` FileName))
  (if _returnvalue
    (if Overwrite
      (`GameplayStatics.SaveGameToSlot` Data FileName :!label _label))
    (else
      (goto _label))))