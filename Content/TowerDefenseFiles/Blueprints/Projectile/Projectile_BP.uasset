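; Tower defense projectile, configured through MakeSetup, that flies to an enemy target and applies a normal, AOE or bounce attack.
; A latent MoveComponentTo glides and turns it toward the target's sampled position, timed by distance over speed, without continuous homing.
; NORMAL damages the target; AOE spawns an AoeZone_BP and emitter.
; BOUNCE damages, then repeats the move toward the nearest not-yet-hit enemy within range until bounces run out.
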(event `self.ReceiveBeginPlay`
  (bind _target (`self.Target`))
  (bind _projectile (`self.Projectile`))
  (bind _target_2 (`self.Target`))
  (bind _relativelocation (`SceneComponent.RelativeLocation` _projectile))
  (bind _location (.location (`self.GetTransform` _target)))
  (`GameplayStatics.PlaySound2D` (`self.Sound`) 1.0 1.0 0.0 null null)
  (`KismetSystemLibrary.Delay` 0.01)
  ;[1 1 1] Move projectile at the given speed. Also rotate the projectile to face the object it goes to
  (if (`KismetSystemLibrary.IsValid` _target) :!label _label
    (`KismetSystemLibrary.MoveComponentTo` _projectile _location (`KismetMathLibrary.FindLookAtRotation` _relativelocation _location) false false (/ (`KismetMathLibrary.VSize` (- _location _relativelocation)) (`self.ProjectileSpeed`)))
    (switch `/Game/TowerDefenseFiles/Blueprints/Auxiliary/AttackType_Enum` (`self.AttackType`)
      (:`NewEnumerator0`
        ;[1 1 1] Deal damage to the enemy (Single Target)
        (if (`KismetSystemLibrary.IsValid` _target_2)
          (`/Game/TowerDefenseFiles/Blueprints/Enemy/BaseEnemy_BP.TakeDamage` _target_2 (`self.Damage`)))
        (`self.K2_DestroyActor`))
      (:`NewEnumerator1`
        ;[1 1 1] Aoe Attack
        (`self.AoeAttack`)
        (`self.K2_DestroyActor`))
      (:`NewEnumerator2`
        ;[1 1 1] Bounce Attack
        (bind _attacknext (`self.BounceAttack`))
        (if _attacknext
          (goto _label))))
    (else
      (`self.K2_DestroyActor`))))

(fn `AoeAttack`
  (bind _returnvalue (`|SpawnActorFromClass` "/Game/TowerDefenseFiles/Blueprints/Auxiliary/AoeZone_BP.AoeZone_BP_C" (`SceneComponent.K2_GetComponentToWorld` (`self.Projectile`)) "Undefined" "OverrideRootScale" null null))
  (set `/Game/TowerDefenseFiles/Blueprints/Auxiliary/AoeZone_BP.Damage` (`self.Damage`) _returnvalue)
  (`SphereComponent.SetSphereRadius` (`/Game/TowerDefenseFiles/Blueprints/Auxiliary/AoeZone_BP.Sphere` _returnvalue) (`self.AoeRadius`) true)
  (`GameplayStatics.SpawnEmitterAtLocation` null (`SceneComponent.K2_GetComponentLocation` (`self.Projectile`)) (struct) (1.0 0.5 1.0)))

(fn `BounceAttack`
  (returns (AttackNext :type Boolean))
  (bind _target (`self.Target`))
  (bind (_indexofminvalue _minvalue) (`KismetMathLibrary.MinOfFloatArray` (`self.BounceDistances`)))
  ;[1 1 1] Damage enemy if possibl (still exists) and decrement number of bounces. Continue with next attack of possible
  (if (`KismetSystemLibrary.IsValid` _target)
    (`/Game/TowerDefenseFiles/Blueprints/Enemy/BaseEnemy_BP.TakeDamage` _target (`self.Damage`))
    (bind _output_get (set `self.NumberOfBounces` (- (`self.NumberOfBounces`) 1)))
    ;[1 1 1] Add enemy to AlreadyAttacked enemies array
    (if (> _output_get 0)
      (`KismetArrayLibrary.Array_Add` (`self.AlreadyAttacked`) (`self.Target`))
      ;[1 1 1] Get all enemies on map and remove the ones that were already attacked
      (`KismetArrayLibrary.Array_Clear` (`self.BounceDistances`))
      (bind _outactors (`GameplayStatics.GetAllActorsOfClass` "/Game/TowerDefenseFiles/Blueprints/Enemy/BaseEnemy_BP.BaseEnemy_BP_C"))
      (bind _output_get_2 (set `self.AllEnemiesOnMap` _outactors))
      (for _array_element (`self.AlreadyAttacked`)
        (`KismetArrayLibrary.Array_RemoveItem` _output_get_2 _array_element))
      ;[1 1 1] Calculate distances from projectile to all enemies
      (for _array_element_2 _output_get_2
        (`KismetArrayLibrary.Array_Add` (`self.BounceDistances`) (`self.GetDistanceTo` self _array_element_2)))
      ;[1 1 1] Get the enemy closest to projectile. If it's in acceptable distance make that the next target to bounce to
      (if (<= _minvalue (`self.MaxBounceDistance`))
        (set `self.Target` (`|GetArrayItem` (`self.AllEnemiesOnMap`) _indexofminvalue))
        (return true)
        (else
          (`self.K2_DestroyActor`)
          (return false)))
      (else
        (`self.K2_DestroyActor`)))
    (else
      (`self.K2_DestroyActor`)))
  (return false))

(fn `MakeSetup`
  (params (ProjectileSpeed :type "Float (double-precision)" :default 900.0) (AttackType :type "/Game/TowerDefenseFiles/Blueprints/Auxiliary/AttackType_Enum Enum" :default "NewEnumerator0") (EnemyTarget :type "/Game/TowerDefenseFiles/Blueprints/Enemy/BaseEnemy_BP Object Reference") (AoeRadius :type "Float (double-precision)") (Damage :type Integer) (NumberOfBounces :type Integer :default 1) (MaxBounceDistance :type "Float (double-precision)" :default 300.0) (NewParam :type "Float (double-precision)" :default 900.0))
  (set `self.ProjectileSpeed` ProjectileSpeed)
  (set `self.AttackType` AttackType)
  (set `self.Target` EnemyTarget)
  (set `self.AoeRadius` AoeRadius)
  (set `self.Damage` Damage)
  (set `self.NumberOfBounces` NumberOfBounces)
  (set `self.MaxBounceDistance` MaxBounceDistance)
  (set `self.ProjectileSpeed` NewParam))

(fn `UserConstructionScript`)