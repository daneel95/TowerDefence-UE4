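; Tower defense projectile that travels to a Target enemy, deals damage and destroys itself, playing a sound on spawn.
; Tick calls a latent MoveComponentTo on the Projectile component, rotating it to face the target, with duration from distance over ProjectileSpeed.
; When the move completes, it applies Damage if the target is still valid, so hits need no collision.
; MakeSetup sets ProjectileSpeed.
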(event `self.ReceiveBeginPlay`
  (`GameplayStatics.PlaySound2D` (`self.Sound`) 1.0 1.0 0.0 null null))

(event `self.ReceiveTick`
  (params (DeltaSeconds :type "Float (single-precision)"))
  (bind _projectile (`self.Projectile`))
  (bind _target (`self.Target`))
  (bind _target_2 (`self.Target`))
  (bind _relativelocation (`SceneComponent.RelativeLocation` _projectile))
  (bind _location (.location (`self.GetTransform` _target_2)))
  ;[1 1 1] Move projectile at the given speed. Also rotate the projectile to face the object it goes to
  (if (`KismetSystemLibrary.IsValid` _target_2)
    (`KismetSystemLibrary.MoveComponentTo` _projectile _location (`KismetMathLibrary.FindLookAtRotation` _relativelocation _location) false false (/ (`KismetMathLibrary.VSize` (- _location _relativelocation)) (`self.ProjectileSpeed`)))
    ;[1 1 1] Deal damage to the enemy
    (if (`KismetSystemLibrary.IsValid` _target)
      (`/Game/TowerDefenseFiles/Blueprints/BaseEnemy_BP.TakeDamage` _target (`self.Damage`)))
    (`self.K2_DestroyActor`)))

(fn `MakeSetup`
  (params (ProjectileSpeed :type "Float (double-precision)" :default 900.0))
  (set `self.ProjectileSpeed` ProjectileSpeed))

(fn `UserConstructionScript`)