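; Tower defense tile that acts as an empty build slot or an automated turret, depending on TurretType.
; Clicking an empty tile shows the turret build widget on the HUD.
; Otherwise, Tick acquires the first Enemy_BP found within Range, keeps it until out of range, and aims TurretTop at it.
; A Delay-gated Fire spawns Projectile_BP at a randomly indexed turret tip at FireRate, passing it Damage and the target.
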(event `self.ReceiveBeginPlay`)

(event `self.ReceiveTick`
  (params (DeltaSeconds :type "Float (single-precision)"))
  (if (`|EnumInequality` (`self.TurretType`) "NewEnumerator0")
    (if (`KismetSystemLibrary.IsValid` (`self.EnemyWithinRange`))
      (`self.CheckEnemyStillInRange`)
      (if (`KismetSystemLibrary.IsValid` (`self.EnemyWithinRange`))
        (`|ExecutionSequence`
          (:`then_0`
            (if (`self.CanFire`)
              (`self.Fire` (`self.TurretTips`))
              (set `self.CanFire` false)
              (`KismetSystemLibrary.Delay` (/ 1.0 (`self.FireRate`)))
              (set `self.CanFire` true)))
          (:`then_1`
            (`SceneComponent.K2_SetWorldRotation` (`self.TurretTop`) (`KismetMathLibrary.FindLookAtRotation` (`SceneComponent.K2_GetComponentLocation` (`self.TurretTop`)) (`SceneComponent.K2_GetComponentLocation` (`/Game/TowerDefenseFiles/Blueprints/Enemy_BP.Cube` (`self.EnemyWithinRange`)))) false false))))
      (else
        (`self.GetEnemyWithinRange`)))))

(event `self.Tile.OnClicked`
  (params (TouchedComponent :type "PrimitiveComponent Object Reference") (ButtonPressed :type "Key Structure"))
  (`KismetSystemLibrary.PrintString` "Hello")
  (if (`|EnumEquality` (`self.TurretType`) "NewEnumerator0")
    (bind _astower_defense_controller (cast `/Game/TowerDefenseFiles/Blueprints/TowerDefenseController` (`GameplayStatics.GetPlayerController` 0)))
    (bind _astower_defense_hud (cast `/Game/TowerDefenseFiles/Blueprints/TowerDefenseHud` (`PlayerController.GetHUD` _astower_defense_controller)))
    (`Widget.SetVisibility` (`/Game/TowerDefenseFiles/Blueprints/TowerDefenseHud.TurretBuildWidget` _astower_defense_hud) "SelfHitTestInvisible")))

(fn `CheckEnemyStillInRange`
  (if (not (< (`self.GetDistanceTo` self (`self.EnemyWithinRange`)) (`self.Range`)))
    (set `self.EnemyWithinRange` null)))

(fn `Fire`
  (params (TurretTips :type "Array of SceneComponent Object Reference"))
  (bind _asstatic_mesh_component (cast `StaticMeshComponent` (`|GetArrayItem` TurretTips (`KismetMathLibrary.RandomIntegerInRange` 0 (`KismetArrayLibrary.Array_Length` TurretTips)))))
  (bind _returnvalue (`|SpawnActorFromClass` "/Game/TowerDefenseFiles/Blueprints/Projectile_BP.Projectile_BP_C" (`KismetMathLibrary.MakeTransform` (`SceneComponent.K2_GetComponentLocation` _asstatic_mesh_component) (struct) (0.1 0.1 0.1)) "Undefined" "OverrideRootScale" null null))
  (`self.SetUpProjectile` _returnvalue))

(fn `GetEnemyWithinRange`
  (bind _outactors (`GameplayStatics.GetAllActorsOfClass` "/Game/TowerDefenseFiles/Blueprints/Enemy_BP.Enemy_BP_C"))
  (for _array_element _outactors
    (if (< (`self.GetDistanceTo` self _array_element) (`self.Range`))
      (set `self.EnemyWithinRange` _array_element)
      (break))))

(fn `SetUpProjectile`
  (params (ProjectileToSetup :type "/Game/TowerDefenseFiles/Blueprints/Projectile_BP Object Reference"))
  (set `/Game/TowerDefenseFiles/Blueprints/Projectile_BP.Damage` (`self.Damage`) ProjectileToSetup)
  (set `/Game/TowerDefenseFiles/Blueprints/Projectile_BP.Target` (`self.EnemyWithinRange`) ProjectileToSetup))

(fn `UserConstructionScript`)