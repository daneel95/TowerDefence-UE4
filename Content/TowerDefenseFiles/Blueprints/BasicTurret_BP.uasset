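; Tower defense turret that automatically shoots at an enemy within range.
; Each Tick it keeps its current Enemy_BP target until that leaves Range, otherwise scanning all enemies and taking the first in range, not the nearest.
; While a target holds, it spawns a scaled-down Projectile_BP at its root, passing it Damage and the Target.
; A CanFire flag and Delay throttle shots to FireRate per second, with debug prints reporting targeting state.
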(event `self.ReceiveBeginPlay`)

(event `self.ReceiveTick`
  (params (DeltaSeconds :type "Float (single-precision)"))
  (if (`KismetSystemLibrary.IsValid` (`self.EnemyWithinRange`))
    (`self.CheckEnemyStillInRange`)
    (if (`KismetSystemLibrary.IsValid` (`self.EnemyWithinRange`))
      (if (`self.CanFire`)
        (`KismetSystemLibrary.PrintString` "Unit within range -> Shooting")
        (bind _returnvalue (`|SpawnActorFromClass` "/Game/TowerDefenseFiles/Blueprints/Projectile_BP.Projectile_BP_C" (`KismetMathLibrary.MakeTransform` (.location (`SceneComponent.GetRelativeTransform` (`self.DefaultSceneRoot`))) (struct) (0.05 0.05 0.05)) "Undefined" "OverrideRootScale" null null))
        (`self.SetUpProjectile` _returnvalue)
        (set `self.CanFire` false)
        (`KismetSystemLibrary.Delay` (/ 1.0 (`self.FireRate`)))
        (set `self.CanFire` true)))
    (else
      (`KismetSystemLibrary.PrintString` "NO UNITS IN RANGE YET")
      (`self.GetEnemyWithinRange`))))

(fn `CheckEnemyStillInRange`
  (if (not (< (`self.GetDistanceTo` self (`self.EnemyWithinRange`)) (`self.Range`)))
    (set `self.EnemyWithinRange` null)))

(fn `GetEnemyWithinRange`
  (bind _outactors (`GameplayStatics.GetAllActorsOfClass` "/Game/TowerDefenseFiles/Blueprints/Enemy_BP.Enemy_BP_C"))
  (for _array_element _outactors
    (if (< (`self.GetDistanceTo` self _array_element) (`self.Range`))
      (set `self.EnemyWithinRange` _array_element)
      (break))))

(fn `SetUpProjectile`
  (params (ProjectileToSetup :type "/Game/TowerDefenseFiles/Blueprints/Projectile_BP Object Reference"))
  (set `/Game/TowerDefenseFiles/Blueprints/Projectile_BP.Damage` (`self.Damage`) ProjectileToSetup)
  (set `/Game/TowerDefenseFiles/Blueprints/Projectile_BP.Target` (`self.EnemyWithinRange`) ProjectileToSetup))

(fn `UserConstructionScript`)