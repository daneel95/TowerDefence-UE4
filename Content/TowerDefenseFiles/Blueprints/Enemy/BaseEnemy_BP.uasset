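; Base tower defense enemy that walks the game mode's checkpoint path, costing the player a life if it reaches the end.
; BeginPlay binds the health bar widget, then loops MoveComponentTo between checkpoints, deriving each move's duration from distance and Speed for constant pace.
; TakeDamage updates the health bar and, at zero health, awards Reward money through TowerDefenseGameMode and destroys the enemy.
; FirstSetup initializes health, speed, reward and type.
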(event `self.ReceiveBeginPlay`
  ;[1 1 1] Set Health Bar
  (bind _asenemy_health_wb (cast `/Game/TowerDefenseFiles/Blueprints/Widgets/EnemyHealth_WB` (`WidgetComponent.GetUserWidgetObject` (`self.Widget`))))
  (set `self.HealthBarWidget` _asenemy_health_wb)
  ;[1 1 1] Get checkpoint and move object to that checkpoint with the given speed
  (`self.GetCheckpoint` :!label _label)
  (`KismetSystemLibrary.MoveComponentTo` (`self.DefaultSceneRoot`) (`self.CheckpointLocation`) (struct) false false (/ (`self.DistanceToTravel`) (`self.Speed`)))
  ;[1 1 1] Check if there is a next checkpoint. If yes repeat
  (set `self.Checkpoint` (+ (`self.Checkpoint`) 1))
  (bind _isnextcheckpoint (`self.CheckNextCheckpoint`))
  (if _isnextcheckpoint
    (goto _label)
    (else
      ;[1 1 1] Else substract life and destroy enemy
      (bind _astower_defense_game_mode (cast `/Game/TowerDefenseFiles/Blueprints/TowerDefenseGameMode` (`GameplayStatics.GetGameMode`)))
      (`/Game/TowerDefenseFiles/Blueprints/TowerDefenseGameMode.SubstractLives` _astower_defense_game_mode 1)
      (`self.K2_DestroyActor`))))

(event `self.ReceiveTick`
  (params (DeltaSeconds :type "Float (single-precision)")))

(fn `CheckNextCheckpoint`
  (returns (IsNextCheckpoint :type Boolean))
  (bind _astower_defense_game_mode (cast `/Game/TowerDefenseFiles/Blueprints/TowerDefenseGameMode` (`GameplayStatics.GetGameMode`)))
  (if (< (`self.Checkpoint`) (`/Game/TowerDefenseFiles/Blueprints/TowerDefenseGameMode.NumberOfCheckpoints` _astower_defense_game_mode))
    (return true)
    (else
      (return false))))

(fn `FirstSetup`
  (params (MaxHealth :type Integer) (Speed :type "Float (double-precision)") (Reward :type Integer) (Type :type "/Game/TowerDefenseFiles/Blueprints/Auxiliary/EnemyType_Enum Enum" :default "NewEnumerator0"))
  (set `self.MaxHealth` MaxHealth)
  (set `self.CurrentHealth` MaxHealth)
  (set `self.Speed` Speed)
  (set `self.Reward` Reward)
  (set `self.Type` Type))

(fn `GetCheckpoint`
  (bind _astower_defense_game_mode (cast `/Game/TowerDefenseFiles/Blueprints/TowerDefenseGameMode` (`GameplayStatics.GetGameMode`)))
  (bind _checkpoint (`/Game/TowerDefenseFiles/Blueprints/TowerDefenseGameMode.GetCheckpoint` _astower_defense_game_mode (`self.Checkpoint`)))
  (bind _output_get (set `self.CheckpointLocation` _checkpoint))
  (set `self.DistanceToTravel` (`KismetMathLibrary.VSize` (- _output_get (`SceneComponent.RelativeLocation` (`self.DefaultSceneRoot`))))))

(fn `TakeDamage`
  (params (Damage :type Integer))
  (bind _output_get (set `self.CurrentHealth` (- (`self.CurrentHealth`) Damage)))
  (`/Game/TowerDefenseFiles/Blueprints/Widgets/EnemyHealth_WB.SetHealth` (`self.HealthBarWidget`) _output_get (`self.MaxHealth`))
  (if (<= (`self.CurrentHealth`) 0)
    (bind _astower_defense_game_mode (cast `/Game/TowerDefenseFiles/Blueprints/TowerDefenseGameMode` (`GameplayStatics.GetGameMode`)))
    (`/Game/TowerDefenseFiles/Blueprints/TowerDefenseGameMode.AddMoney` _astower_defense_game_mode (`self.Reward`))
    (`self.K2_DestroyActor`)))

(fn `UserConstructionScript`)