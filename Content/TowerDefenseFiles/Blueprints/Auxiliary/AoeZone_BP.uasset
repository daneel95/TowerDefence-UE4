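; AoeZone_BP is a short-lived area-of-effect damage zone for the tower defense game.
; After a tiny delay on BeginPlay, it gathers BaseEnemy_BP actors overlapping its Sphere and calls TakeDamage on each with its Damage value.
; It then destroys itself, so each spawn delivers one damage burst.
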(event `self.ReceiveBeginPlay`
  (`KismetSystemLibrary.Delay` 0.01)
  (bind _output_get (set `self.EnemiesArray` (`PrimitiveComponent.GetOverlappingActors` (`self.Sphere`) "/Game/TowerDefenseFiles/Blueprints/Enemy/BaseEnemy_BP.BaseEnemy_BP_C")))
  (for _array_element _output_get
    (bind _asbase_enemy_bp (cast `/Game/TowerDefenseFiles/Blueprints/Enemy/BaseEnemy_BP` _array_element))
    (if (`KismetSystemLibrary.IsValid` _asbase_enemy_bp)
      (`/Game/TowerDefenseFiles/Blueprints/Enemy/BaseEnemy_BP.TakeDamage` _asbase_enemy_bp (`self.Damage`))))
  (`self.K2_DestroyActor`))

(fn `UserConstructionScript`)