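; Tower defense enemy actor that walks a checkpoint path and pays a money reward when killed.
; Checkpoint positions come from TowerDefenseGameMode, and a looping MoveComponentTo moves the root between them, timed as distance over Speed for constant pace.
; It destroys itself after the last checkpoint.
; TakeDamage updates the EnemyHealth_WB health bar and, at zero health, adds Reward to the game mode's money and destroys the enemy.
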(event `self.ReceiveBeginPlay`
  (bind _asenemy_health_wb (cast `/Game/TowerDefenseFiles/Blueprints/EnemyHealth_WB` (`WidgetComponent.GetUserWidgetObject` (`self.Widget`))))
  (set `self.HealthBarWidget` _asenemy_health_wb)
  (`self.GetCheckpoint` :!label _label)
  (`KismetSystemLibrary.MoveComponentTo` (`self.DefaultSceneRoot`) (`self.CheckpointLocation`) (struct) false false (/ (`self.DistanceToTravel`) (`self.Speed`)))
  (set `self.Checkpoint` (+ (`self.Checkpoint`) 1))
  (bind _isnextcheckpoint (`self.CheckNextCheckpoint`))
  (if _isnextcheckpoint
    (goto _label)
    (else
      (`self.K2_DestroyActor`))))

(event `self.ReceiveTick`
  (params (DeltaSeconds :type "Float (single-precision)")))

(fn `CheckNextCheckpoint`
  (returns (IsNextCheckpoint :type Boolean))
  (bind _astower_defense_game_mode (cast `/Game/TowerDefenseFiles/Blueprints/TowerDefenseGameMode` (`GameplayStatics.GetGameMode`)))
  (if (< (`self.Checkpoint`) (`/Game/TowerDefenseFiles/Blueprints/TowerDefenseGameMode.NumberOfCheckpoints` _astower_defense_game_mode))
    (return true)
    (else
      (return false))))

(fn `GetCheckpoint`
  (bind _astower_defense_game_mode (cast `/Game/TowerDefenseFiles/Blueprints/TowerDefenseGameMode` (`GameplayStatics.GetGameMode`)))
  (bind _checkpoint (`/Game/TowerDefenseFiles/Blueprints/TowerDefenseGameMode.GetCheckpoint` _astower_defense_game_mode (`self.Checkpoint`)))
  (bind _output_get (set `self.CheckpointLocation` _checkpoint))
  (set `self.DistanceToTravel` (`KismetMathLibrary.VSize` (- _output_get (`SceneComponent.RelativeLocation` (`self.DefaultSceneRoot`))))))

(fn `TakeDamage`
  (params (Damage :type Integer))
  (bind _output_get (set `self.CurrentHealth` (- (`self.CurrentHealth`) Damage)))
  (`/Game/TowerDefenseFiles/Blueprints/EnemyHealth_WB.SetHealth` (`self.HealthBarWidget`) _output_get (`self.MaxHealth`))
  (if (<= (`self.CurrentHealth`) 0)
    (bind _astower_defense_game_mode (cast `/Game/TowerDefenseFiles/Blueprints/TowerDefenseGameMode` (`GameplayStatics.GetGameMode`)))
    (`/Game/TowerDefenseFiles/Blueprints/TowerDefenseGameMode.AddMoney` _astower_defense_game_mode (`self.Reward`))
    (`self.K2_DestroyActor`)))

(fn `UserConstructionScript`)